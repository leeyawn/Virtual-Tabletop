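; Blueprint function library of small math helpers for rounding, grid snapping and parity checks.
; RoundToMultiple raises positive integers to the next multiple using modulo, but its negative branch tests an absolute-value remainder, so negative inputs round incorrectly.
; SnapVectorToVector grid-snaps each axis of one vector by the matching component of another.
; IsFloatEven and IsIntegerEven test for a zero remainder when divided by two.
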(fn RoundtoMultiple
  (params (NumToRound :type Integer) (Multiple :type Integer))
  (bind _returnvalue (Math|Integer|Absolute(Integer) NumToRound))
  (if (== Multiple 0)
    (LocalVariables|SetReturnValue NumToRound :!label _label)
    (else
      (bind _output_get (LocalVariables|SetRemainder (Math|Integer|%(Integer) _returnvalue Multiple)))
      (if (== _output_get 0)
        (goto _label)
        (elif (< _output_get 0)
          (LocalVariables|SetReturnValue (* (- _returnvalue _output_get) -1))
          (else
            (LocalVariables|SetReturnValue (- (+ NumToRound Multiple) _output_get)))))))
  (return (LocalVariables|GetReturnValue)))

(fn SnapVectortoVector
  (params (V1 :type Vector) (V2 :type Vector))
  (return (Math|Vector|MakeVector (Math|Float|SnapToGrid(Float) (.x V1) (.x V2)) (Math|Float|SnapToGrid(Float) (.y V1) (.y V2)) (Math|Float|SnapToGrid(Float) (.z V1) (.z V2)))))

(fn IsFloatEven
  (params (Float :type Float%20%28double-precision%29))
  (return (== (Math|Float|%(Float) Float 2.0) 0.0)))

(fn IsIntegerEven
  (params (Integer :type Integer))
  (return (== (Math|Integer|%(Integer) Integer 2) 0)))