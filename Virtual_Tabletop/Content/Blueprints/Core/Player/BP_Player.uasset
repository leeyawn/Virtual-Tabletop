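; BP_Player is a player camera pawn that moves, rotates and zooms through Enhanced Input.
; It registers IMC_Default when the controller changes, then seeds the desired zoom and rotation and caps FPS at 60 on BeginPlay.
; Zoom and rotate inputs adjust those targets, which Tick interpolates onto spring arm length and actor rotation.
; Movement uses AddMovementInput along control-rotation axes, leaving the older location-interpolation logic unused.
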(event Input|EnhancedActionEvents|EnhancedInputActionIA_Camera_Zoom
  (params (ActionValue :type Float%20%28double-precision%29) (ElapsedSeconds :type Float%20%28double-precision%29) (TriggeredSeconds :type Float%20%28double-precision%29) (InputAction :type Input%20Action%20Object%20Reference :default "/Game/Blueprints/Core/Player/Inputs/IA_Camera_Zoom.IA_Camera_Zoom"))
  ;[0.15 0.15 0.15 0.5] Zoom Camera Pawn
  (Variables|Zoom|SetZoomDesired (Math|Float|Clamp(Float) (+ (* ActionValue (Variables|Zoom|GetZoomSpeed)) (Variables|Zoom|GetZoomDesired)) (Variables|Zoom|GetZoomMin) (Variables|Zoom|GetZoomMax))))

(event Input|EnhancedActionEvents|EnhancedInputActionIA_Camera_Rotate
  (params (ActionValue :type Float%20%28double-precision%29) (ElapsedSeconds :type Float%20%28double-precision%29) (TriggeredSeconds :type Float%20%28double-precision%29) (InputAction :type Input%20Action%20Object%20Reference :default "/Game/Blueprints/Core/Player/Inputs/IA_Camera_Rotate.IA_Camera_Rotate"))
  ;[0.15 0.15 0.15 0.5] Rotate Camera Pawn
  (Variables|Rotation|SetRotationDesired (Math|Rotator|CombineRotators (Variables|Rotation|GetRotationDesired) (Math|Rotator|MakeRotator 0.0 0.0 (* ActionValue (Variables|Rotation|GetRotationSpeed))))))

(event Input|EnhancedActionEvents|EnhancedInputActionIA_Camera_Move
  (params (ActionValue :type Vector%202D%20Structure) (ElapsedSeconds :type Float%20%28double-precision%29) (TriggeredSeconds :type Float%20%28double-precision%29) (InputAction :type Input%20Action%20Object%20Reference :default "/Game/Blueprints/Core/Player/Inputs/IA_Camera_Move.IA_Camera_Move"))
  (bind _returnvalue (Math|Vector2D|Normalize2D ActionValue))
  (bind _returnvalue_2 (Pawn|GetControlRotation :!class /Script/Engine.Pawn))
  ;[0.15 0.15 0.15 0.5] Move Camera Pawn
  (Pawn|Input|AddMovementInput (Math|Vector|GetForwardVector (Math|Rotator|MakeRotator 0.0 0.0 (.yaw (Pawn|GetControlRotation :!class /Script/Engine.Pawn)))) (.x _returnvalue) false)
  (Pawn|Input|AddMovementInput (Math|Vector|GetRightVector (Math|Rotator|MakeRotator (.roll _returnvalue_2) 0.0 (.yaw _returnvalue_2))) (.y _returnvalue) false))

(event EventTick
  (params (DeltaSeconds :type Float%20%28single-precision%29))
  (Variables|Default|SetDeltaSeconds DeltaSeconds)
  (CallFunction|UpdateCameraView))

(event EventBeginPlay
  (CallFunction|InitializeCameraView))

(event EventControllerChanged
  (params (OldController :type Controller%20Object%20Reference) (NewController :type Controller%20Object%20Reference))
  (bind _asbp_pc (Utilities|Casting|CastToBP_PC NewController))
  (Utilities|IsValid (PlayerController|LocalPlayerSubsystems|GetEnhancedInputLocalPlayerSubsystem _asbp_pc)
    (:Is%20Valid
      (Input|AddMappingContext (PlayerController|LocalPlayerSubsystems|GetEnhancedInputLocalPlayerSubsystem _asbp_pc) "/Game/Blueprints/Core/Player/Inputs/IMC_Default.IMC_Default" 0 "(bIgnoreAllPressedKeysUntilRelease=True,bForceImmediately=False,bNotifyUserSettings=False)"))))

(fn ConstructionScript)

(fn UpdateCameraView
  (bind _springarm (Variables|Default|GetSpringArm))
  (Variables|/Script/Engine.SpringArmComponent|SetTargetArmLength _springarm (Math|Interpolation|FInterpTo (Variables|/Script/Engine.SpringArmComponent|GetTargetArmLength _springarm) (Variables|Zoom|GetZoomDesired) (Variables|Default|GetDeltaSeconds) (Variables|Zoom|GetZoomInterp)))
  (Transformation|SetActorRotation (Math|Interpolation|RInterpTo (Transformation|GetActorRotation) (Variables|Rotation|GetRotationDesired) (Variables|Default|GetDeltaSeconds) (Variables|Rotation|GetRotationInterp))))

(fn InitializeCameraView
  (Variables|Location|SetLocationDesired (Transformation|GetActorLocation))
  (Variables|Zoom|SetZoomDesired (Variables|/Script/Engine.SpringArmComponent|GetTargetArmLength (Variables|Default|GetSpringArm)))
  (Variables|Rotation|SetRotationDesired (Transformation|GetActorRotation))
  (Development|ExecuteConsoleCommand "t.MaxFps 60" 0))

(fn InitializeKeyboardInputs)

(fn OldMovement
  (params (A :type Vector%202D%20Structure))
  (bind _returnvalue (Math|Vector2D|Normalize2D A))
  (Variables|Location|SetLocationDesired (+ (* (Transformation|GetActorForwardVector) (* (.x _returnvalue) (Variables|Location|GetLocationSpeed))) (Variables|Location|GetLocationDesired) (* (Transformation|GetActorRightVector) (* (.y _returnvalue) (Variables|Location|GetLocationSpeed)))))
  (return (.y _returnvalue) (.x _returnvalue)))