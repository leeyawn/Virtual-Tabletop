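; BP_PC is a player controller that provides in-game text chat.
; On BeginPlay it shows the mouse cursor and, for the local controller, creates the W_ChatPanel widget, whose input box takes keyboard focus on Enter.
; SR_SubmitChat loops over the GameState PlayerArray and relays the sender name and message to each player's BP_PC through OC_UpdateChat, which updates that player's panel.
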(event Custom|SR_SubmitChat
  (params (PlayerName :type Text) (ChatMessage :type Text))
  (for _array_element (Variables|/Script/Engine.GameStateBase|GetPlayerArray (Game|GetGameState))
    (bind _asbp_pc (Utilities|Casting|CastToBP_PC (Game|GetPlayerController _array_element)))
    (CallFunction|OCUpdateChat _asbp_pc PlayerName ChatMessage)))

(event Custom|OC_UpdateChat
  (params (PlayerName :type Text) (ChatMessgae :type Text))
  (bind _w_chatpanel (Variables|Default|GetW_ChatPanel)
    (:then
      (Default|UpdateChat _w_chatpanel PlayerName ChatMessgae))
    (:else)))

(event EventBeginPlay
  (Variables|Default|SetbShowMouseCursor true)
  (if (Pawn|IsLocalPlayerController)
    (bind _returnvalue (UserInterface|CreateWidget "/Game/Blueprints/ChatBox/W_ChatPanel.W_ChatPanel_C" self))
    (bind _output_get (Variables|Default|SetW_ChatPanel _returnvalue))
    (UserInterface|Viewport|AddtoViewport _output_get 1)))

(event Input|KeyboardEvents|Enter
  (params (Key :type Key%20Structure :default "None"))
  (:Pressed
    (bind _w_chatpanel (Variables|Default|GetW_ChatPanel)
      (:then
        (Widget|SetKeyboardFocus (Variables|/Game/Blueprints/ChatBox/W_ChatPanel.W_ChatPanel_C|GetChat_InputBox _w_chatpanel)))
      (:else))))

(fn ConstructionScript)