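; FL_MathLibrary is a math function library with one helper, RoundToMultiple, which rounds a number up to a given multiple.
; A zero multiple or exact multiple returns the input unchanged; otherwise it adds the multiple minus the remainder of the absolute input.
; The negative-handling branch tests that remainder rather than the input, so it appears unreachable, and negative inputs can land off-multiple.
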(fn RoundtoMultiple
  (params (NumToRound :type Integer) (Multiple :type Integer))
  (bind _returnvalue (Math|Integer|Absolute(Integer) NumToRound))
  (if (== Multiple 0)
    (LocalVariables|SetReturnValue NumToRound :!label _label)
    (else
      (bind _output_get (LocalVariables|SetRemainder (Math|Integer|%(Integer) _returnvalue Multiple)))
      (if (== _output_get 0)
        (goto _label)
        (elif (< _output_get 0)
          (LocalVariables|SetReturnValue (* (- _returnvalue _output_get) -1))
          (else
            (LocalVariables|SetReturnValue (- (+ NumToRound Multiple) _output_get)))))))
  (return (LocalVariables|GetReturnValue)))